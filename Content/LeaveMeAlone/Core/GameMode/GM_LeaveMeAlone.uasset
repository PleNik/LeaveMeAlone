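; LeaveMeAlone game mode that runs a match countdown and holds logic for a death screen.
; A looping one-second timer from BeginPlay decrements GameTime, then at zero stops, shows the game-over widget and enables the mouse cursor.
; HealthEnd similarly counts down DeadTime to show the death widget.
; The health check meant to schedule HealthEnd is unconnected and never runs, leaving the death screen untriggered here.
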(event `self.ReceiveBeginPlay`
  (bind _returnvalue (`KismetSystemLibrary.K2_SetTimerDelegate` (delegate `GameTimer`) 1.0 true))
  (set `self.GameTimerHandle` _returnvalue))

(event `GameTimer`
  (bind _result (`/Engine/EditorBlueprintResources/StandardMacros.DecrementInt` (`self.GameTime`))
    (:`  `
      (if (== _result 0)
        (`KismetSystemLibrary.K2_ClearAndInvalidateTimerHandle` (`self.GameTimerHandle`))
        (bind _returnvalue (`|CreateWidget` "/Game/LeaveMeAlone/Widgets/WBP_GameOver.WBP_GameOver_C"))
        (bind _output_get (set `self.TimerOverWidget` _returnvalue))
        (`UserWidget.AddToViewport` _output_get 0)
        (set `PlayerController.bShowMouseCursor` true (`GameplayStatics.GetPlayerController` 0))))))

(event `HealthEnd`
  ;[1 1 1] Screen Of Death
  (bind _result (`/Engine/EditorBlueprintResources/StandardMacros.DecrementInt` (`self.DeadTime`))
    (:`  `
      (if (== _result 0)
        (`KismetSystemLibrary.K2_ClearAndInvalidateTimerHandle` (`self.DeadTimerHandle`))
        (bind _returnvalue (`|CreateWidget` "/Game/LeaveMeAlone/Widgets/WBP_Dead.WBP_Dead_C"))
        (bind _output_get (set `self.DeadWidget` _returnvalue))
        (`UserWidget.AddToViewport` _output_get 0)
        (set `PlayerController.bShowMouseCursor` true (`GameplayStatics.GetPlayerController` 0))))))

(fn `UserConstructionScript`)